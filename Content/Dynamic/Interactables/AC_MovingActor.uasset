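; Actor component that moves its owner back and forth between its starting location and the location of a referenced EndActor.
; BeginPlay caches both positions and starts a looping timer that steps a lerp alpha, flipping the step's sign at either end.
; An alternative speed-based Tick mover with target swapping is gated by IsMoving, which is set only in disconnected setup nodes alongside the EndActor validity check.
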(event Custom|SetTargetPosition
  ;[1 1 1] Comment
  (if (<= (Math|Vector|Distance(Vector) (Transformation|GetActorLocation (Components|GetOwner)) (Variables|Default|GetStartPos)) 2.0)
    (Variables|Default|SetTargetPos (Variables|Default|GetEndPos))
    (else
      (Variables|Default|SetTargetPos (Variables|Default|GetStartPos)))))

(event Custom|ChangeLerpAlphaValue
  (bind _output_get (Variables|Default|SetCurrentPosLength (+ (Variables|Default|GetCurrentPosLength) (Variables|Default|GetValuetoaddtoalpha))))
  (if (>= _output_get 1.0)
    (Variables|Default|SetValuetoaddtoalpha (* (Variables|Default|GetValuetoaddtoalpha) -1.0))
    (elif (< (Variables|Default|GetCurrentPosLength) 0.0)
      (Variables|Default|SetValuetoaddtoalpha (* (Variables|Default|GetValuetoaddtoalpha) -1.0))))
  (Transformation|SetActorLocation (Components|GetOwner) (Math|Vector|Lerp(Vector) (Variables|Default|GetStartPos) (Variables|Default|GetTargetPos) (Variables|Default|GetCurrentPosLength)) false false))

(event EventBeginPlay
  (Variables|Default|SetStartPos (Transformation|GetActorLocation (Components|GetOwner)))
  (Variables|Default|SetTargetPos (Transformation|GetActorLocation (Variables|Default|GetEndActor)))
  (Utilities|Time|SetTimerbyEvent (delegate Custom|ChangeLerpAlphaValue) 0.03 true))

(event EventTick
  (params (DeltaSeconds :type Float%20%28single-precision%29))
  ;[1 1 1] Comment
  (if (Variables|Default|GetbIsMoving)
    (|CalculatePositionLength DeltaSeconds)
    (Transformation|SetActorLocation (Components|GetOwner) (Math|Vector|Lerp(Vector) (Transformation|GetActorLocation (Components|GetOwner)) (Variables|Default|GetTargetPos) (Math|Float|Clamp(Float) (Variables|Default|GetCurrentPosLength))) false false)
    (if (>= (Math|Float|Clamp(Float) (Variables|Default|GetCurrentPosLength)) 0.1)
      (CallFunction|SetTargetPosition)
      (Variables|Default|SetCurrentPosLength 0.0))))